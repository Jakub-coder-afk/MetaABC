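; BP_MainCharacter is the main character Blueprint, adding debug keys that exercise enemy AI on top of its parent class.
; The keys emit a noise at the character's location, report a damage stimulus against a BP_MainEnemy, or set that enemy's AIC_BaseEnemy controller to passive.
; The enemy is found with GetActorOfClass, so only one instance is targeted.
; BeginPlay and construction defer to the parent, and IA_Dum is an empty input stub.
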(event Input|EnhancedActionEvents|EnhancedInputActionIA_Dum
  (params (ActionValue :type Boolean) (ElapsedSeconds :type Float%20%28double-precision%29) (TriggeredSeconds :type Float%20%28double-precision%29) (InputAction :type Input%20Action%20Object%20Reference :default "/Game/ThirdPerson/Input/Actions/IA_Dum.IA_Dum")))

(event EventBeginPlay
  (|CallParentFunction))

(event Collision|EventActorBeginOverlap
  (params (OtherActor :type Actor%20Object%20Reference)))

(event EventTick
  (params (DeltaSeconds :type Float%20%28single-precision%29)))

(event Input|KeyboardEvents|DebugKeyP
  (params (Key :type Key%20Structure) (ActionValue :type Input%20Action%20Value%20Structure))
  (:Pressed
    (bind _returnvalue (Actor|GetActorOfClass "/Game/TEB_07_06/Characters/BP_MainEnemy.BP_MainEnemy_C"))
    (bind _asaic_base_enemy (Utilities|Casting|CastToAIC_BaseEnemy (AI|GetAIController _returnvalue)))
    (Default|SetStateasPassive _asaic_base_enemy)))

(event Input|KeyboardEvents|DebugKeyO
  (params (Key :type Key%20Structure) (ActionValue :type Input%20Action%20Value%20Structure))
  (:Pressed
    (bind _returnvalue (Actor|GetActorOfClass "/Game/TEB_07_06/Characters/BP_MainEnemy.BP_MainEnemy_C"))
    (Class|AISenseDamage|ReportDamageEvent _returnvalue self 5.0 (Transformation|GetActorLocation) "0, 0, 0" "None")))

(event Input|KeyboardEvents|DebugKeyN
  (params (Key :type Key%20Structure) (ActionValue :type Input%20Action%20Value%20Structure))
  (:Pressed
    (Class|Actor|MakeNoise 1.0 self (Transformation|GetActorLocation) 0.0 "None")))

(fn ConstructionScript
  (|CallParentFunction))